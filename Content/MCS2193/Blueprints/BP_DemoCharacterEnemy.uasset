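; BP_DemoCharacterEnemy is a demo enemy that reports pawns it sees to its AI controller's Blackboard.
; When PawnSensing sees a pawn, a class check gates writing it to the Player key and setting SeePlayer true.
; A one-second retriggerable delay, restarted on each sighting, then writes false as a bool to the Player key, leaving SeePlayer untouched.
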(event OnSeePawn(PawnSensing)
  (params (Pawn :type Pawn%20Object%20Reference))
  (bind _self self)
  (bind _returnvalue (AI|GetAIController _self))
  (Variables|Default|SetPawn Pawn)
  (Utilities|FlowControl|Sequence
    (:then_0
      (if (Utilities|ClassIsChildOf (Utilities|GetClass Pawn) 0)
        (AI|Components|Blackboard|SetValueasObject (AI|GetBlackboard _returnvalue) (Utilities|Name|MakeLiteralName "Player") (Variables|Default|GetPawn))
        (AI|Components|Blackboard|SetValueasBool (AI|GetBlackboard _returnvalue) (Utilities|Name|MakeLiteralName "SeePlayer") true)))
    (:then_1
      (Utilities|FlowControl|RetriggerableDelay 1.0)
      (AI|Components|Blackboard|SetValueasBool (AI|GetBlackboard (AI|GetAIController self)) (Utilities|Name|MakeLiteralName "Player") false))))

(fn ConstructionScript)