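; Health Blueprint that tracks a current health value, set to the maximum on BeginPlay.
; Damage subtracts the incoming amount without clamping, calls OnDamage, and also calls OnDead when health is zero or below.
; GetCurrentHealth exposes the value, and pressing X applies a fixed amount of damage.
; The OnDamage and OnDead events in the event graph are empty.
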(event Custom|OnDamage)

(event Custom|OnDead)

(event EventBeginPlay
  (Variables|Default|SetCurrentHealth (Variables|Default|GetMaxHealth)))

(event EventTick
  (params (DeltaSeconds :type Float%20%28single-precision%29)))

(event Input|KeyboardEvents|X
  (params (Key :type Key%20Structure :default "None"))
  (:Pressed
    (CallFunction|Damage 10)))

(fn Damage
  (params (DamageTaken :type Integer))
  (bind _output_get (Variables|Default|SetCurrentHealth (- (Variables|Default|GetCurrentHealth) DamageTaken)))
  (Default|CallOnDamage)
  (if (<= _output_get 0)
    (Default|CallOnDead)))

(fn GetCurrentHealth
  (return (Variables|Default|GetCurrentHealth)))